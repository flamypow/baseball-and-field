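; Player one's drone in a local two-player game, constantly moving forward along four directions.
; Enhanced Input presses turn it without allowing reversals, or fire a timed bullet when matching the current heading, one at a time via BulletInPlay.
; It also forwards player two's input to the BP_Player2Drone found by tag.
; Overlapping a PlayerTwo-tagged actor destroys both, and its own destruction triggers CallPlayerDestroyed.
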(event `self.ReceiveBeginPlay`
  (bind _outactors (`GameplayStatics.GetAllActorsWithTag` "PlayerTwo"))
  (bind _asbp_player_2drone (cast `/Game/Blueprints/BP_Player2Drone` (`|GetArrayItem` _outactors)))
  (set `self.Player2` _asbp_player_2drone)
  ;[1 1 1] Add Input Controls
  (bind _asplayer_controller (cast `PlayerController` (`self.GetController`)))
  (bind _returnvalue (pcsubsystem `EnhancedInputLocalPlayerSubsystem` _asplayer_controller))
  (`/Engine/EditorBlueprintResources/StandardMacros.IsValid` _returnvalue
    (:`Is Valid`
      (`EnhancedInputSubsystemInterface.AddMappingContext` _returnvalue "/Game/Input/IMC_Drone1.IMC_Drone1" 0 (struct)))))

(event `self.ReceiveTick`
  (params (DeltaSeconds :type "Float (single-precision)"))
  (`self.K2_SetActorLocation` (+ (`self.K2_GetActorLocation`) (* (`self.speed`) (`GameplayStatics.GetWorldDeltaSeconds`) (`self.GetActorForwardVector`)))))

(event `EnhancedInput|/Game/Input/IA_UpPressedP1`
  (params (ActionValue :type Boolean) (ElapsedSeconds :type "Float (double-precision)") (TriggeredSeconds :type "Float (double-precision)") (InputAction :type "InputAction Object Reference" :default "/Game/Input/IA_UpPressedP1.IA_UpPressedP1"))
  (:`Triggered`
    (if (== (`self.K2_GetActorRotation`) (struct) :`ErrorTolerance` 1.0)
      (if (not (`self.BulletInPlay`))
        (set `self.BulletInPlay` true)
        (bind _returnvalue (`|SpawnActorFromClass` "/Game/Blueprints/BP_PlayerDroneBullet.BP_PlayerDroneBullet_C" (`self.GetTransform`) "AlwaysSpawn" "MultiplyWithRoot" null null))
        (`self.SetOwner` _returnvalue self)
        (`KismetSystemLibrary.Delay` (`self.Duration`))
        (`self.K2_DestroyActor` _returnvalue))
      (elif (not (== (`self.K2_GetActorRotation`) (struct :`Yaw` 180.0) :`ErrorTolerance` 1.0))
        (`self.K2_SetActorRotation` (struct))))))

(event `EnhancedInput|/Game/Input/IA_DownPressedP1`
  (params (ActionValue :type Boolean) (ElapsedSeconds :type "Float (double-precision)") (TriggeredSeconds :type "Float (double-precision)") (InputAction :type "InputAction Object Reference" :default "/Game/Input/IA_DownPressedP1.IA_DownPressedP1"))
  (:`Triggered`
    (if (== (`self.K2_GetActorRotation`) (struct :`Yaw` 180.0) :`ErrorTolerance` 1.0)
      (if (not (`self.BulletInPlay`))
        (set `self.BulletInPlay` true)
        (bind _returnvalue (`|SpawnActorFromClass` "/Game/Blueprints/BP_PlayerDroneBullet.BP_PlayerDroneBullet_C" (`self.GetTransform`) "AlwaysSpawn" "MultiplyWithRoot" null null))
        (`self.SetOwner` _returnvalue self)
        (`KismetSystemLibrary.Delay` (`self.Duration`))
        (`self.K2_DestroyActor` _returnvalue))
      (elif (not (== (`self.K2_GetActorRotation`) (struct) :`ErrorTolerance` 1.0))
        (`self.K2_SetActorRotation` (struct :`Yaw` 180.0))))))

(event `EnhancedInput|/Game/Input/IA_LeftPressedP1`
  (params (ActionValue :type Boolean) (ElapsedSeconds :type "Float (double-precision)") (TriggeredSeconds :type "Float (double-precision)") (InputAction :type "InputAction Object Reference" :default "/Game/Input/IA_LeftPressedP1.IA_LeftPressedP1"))
  (:`Triggered`
    (if (== (`self.K2_GetActorRotation`) (struct :`Yaw` 270.0) :`ErrorTolerance` 1.0)
      (if (not (`self.BulletInPlay`))
        (set `self.BulletInPlay` true)
        (bind _returnvalue (`|SpawnActorFromClass` "/Game/Blueprints/BP_PlayerDroneBullet.BP_PlayerDroneBullet_C" (`self.GetTransform`) "AlwaysSpawn" "MultiplyWithRoot" null null))
        (`self.SetOwner` _returnvalue self)
        (`KismetSystemLibrary.Delay` (`self.Duration`))
        (`self.K2_DestroyActor` _returnvalue))
      (elif (not (== (`self.K2_GetActorRotation`) (struct :`Yaw` 90.0) :`ErrorTolerance` 1.0))
        (`self.K2_SetActorRotation` (struct :`Yaw` 270.0))))))

(event `EnhancedInput|/Game/Input/IA_RightPressedP1`
  (params (ActionValue :type Boolean) (ElapsedSeconds :type "Float (double-precision)") (TriggeredSeconds :type "Float (double-precision)") (InputAction :type "InputAction Object Reference" :default "/Game/Input/IA_RightPressedP1.IA_RightPressedP1"))
  (:`Triggered`
    (if (== (`self.K2_GetActorRotation`) (struct :`Yaw` 90.0) :`ErrorTolerance` 1.0)
      (if (not (`self.BulletInPlay`))
        (set `self.BulletInPlay` true)
        (bind _returnvalue (`|SpawnActorFromClass` "/Game/Blueprints/BP_PlayerDroneBullet.BP_PlayerDroneBullet_C" (`self.GetTransform`) "AlwaysSpawn" "MultiplyWithRoot" null null))
        (`self.SetOwner` _returnvalue self)
        (`KismetSystemLibrary.Delay` (`self.Duration`))
        (`self.K2_DestroyActor` _returnvalue))
      (elif (not (== (`self.K2_GetActorRotation`) (struct :`Yaw` 270.0) :`ErrorTolerance` 1.0))
        (`self.K2_SetActorRotation` (struct :`Yaw` 90.0))))))

(event `BulletDestroyed`
  (set `self.BulletInPlay` false))

(event `self.ReceiveDestroyed`
  (set `self.IsDestroyed` true)
  (`self.PlayerDestroyed`))

(event `EnhancedInput|/Game/Input/IA_DownPressedP2`
  (params (ActionValue :type Boolean) (ElapsedSeconds :type "Float (double-precision)") (TriggeredSeconds :type "Float (double-precision)") (InputAction :type "InputAction Object Reference" :default "/Game/Input/IA_DownPressedP2.IA_DownPressedP2"))
  (:`Triggered`
    (`/Game/Blueprints/BP_Player2Drone.P2Down` (`self.Player2`))))

(event `EnhancedInput|/Game/Input/IA_LeftPressedP2`
  (params (ActionValue :type Boolean) (ElapsedSeconds :type "Float (double-precision)") (TriggeredSeconds :type "Float (double-precision)") (InputAction :type "InputAction Object Reference" :default "/Game/Input/IA_LeftPressedP2.IA_LeftPressedP2"))
  (:`Triggered`
    (`/Game/Blueprints/BP_Player2Drone.P2Left` (`self.Player2`))))

(event `EnhancedInput|/Game/Input/IA_RightPressedP2`
  (params (ActionValue :type Boolean) (ElapsedSeconds :type "Float (double-precision)") (TriggeredSeconds :type "Float (double-precision)") (InputAction :type "InputAction Object Reference" :default "/Game/Input/IA_RightPressedP2.IA_RightPressedP2"))
  (:`Triggered`
    (`/Game/Blueprints/BP_Player2Drone.P2Right` (`self.Player2`))))

(event `EnhancedInput|/Game/Input/IA_UpPressedP2`
  (params (ActionValue :type Boolean) (ElapsedSeconds :type "Float (double-precision)") (TriggeredSeconds :type "Float (double-precision)") (InputAction :type "InputAction Object Reference" :default "/Game/Input/IA_UpPressedP2.IA_UpPressedP2"))
  (:`Triggered`
    (`/Game/Blueprints/BP_Player2Drone.P2Up` (`self.Player2`))))

(event `self.Capsule.OnComponentBeginOverlap`
  (params (OverlappedComponent :type "PrimitiveComponent Object Reference") (OtherActor :type "Actor Object Reference") (OtherComp :type "PrimitiveComponent Object Reference") (OtherBodyIndex :type Integer) (bFromSweep :type Boolean) (SweepResult :type "HitResult Structure (by ref)"))
  (if (`self.ActorHasTag` OtherActor "PlayerTwo")
    (`self.K2_DestroyActor` OtherActor)
    (`self.K2_DestroyActor`)))

(fn `UserConstructionScript`)
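; Bat actor with a Cylinder component and an early spacebar-driven windup rotation.
; While IA_SpaceBar is Ongoing, it sets the actor's pitch to the Cylinder's relative pitch plus WindupSpeed scaled by delta time, and prints a debug string.
; Because it reads component-relative pitch but writes actor rotation, the pitch does not accumulate.
; The branch is hardcoded true, leaving the pitch-limit check unconnected and the pitch printout unreachable.
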(event `EnhancedInput|/Game/Input/IA_SpaceBar`
  (params (ActionValue :type Boolean) (ElapsedSeconds :type "Float (double-precision)") (TriggeredSeconds :type "Float (double-precision)") (InputAction :type "InputAction Object Reference" :default "/Game/Input/IA_SpaceBar.IA_SpaceBar"))
  (bind (_relativerotation_roll _relativerotation_pitch) (`KismetMathLibrary.BreakRotator` (`SceneComponent.RelativeRotation` (`self.Cylinder`))))
  (:`Ongoing`
    (if true
      (`KismetSystemLibrary.PrintString` "Hello")
      (`self.K2_SetActorRotation` (`KismetMathLibrary.MakeRotator` 0.0 (+ _relativerotation_pitch (* (`self.WindupSpeed`) (`GameplayStatics.GetWorldDeltaSeconds`)))))
      (else
        (`KismetSystemLibrary.PrintString` (`KismetStringLibrary.Conv_DoubleToString` _relativerotation_pitch))))))

(fn `UserConstructionScript`)
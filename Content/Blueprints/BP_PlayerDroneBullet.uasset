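; BP_PlayerDroneBullet is a projectile fired by BP_PlayerDrone that destroys actors tagged as Player Two or Player Two's bullets.
; Each tick it moves forward without sweeping and copies its owner's rotation, so it steers with the owner while in flight.
; A capsule overlap with either tag destroys both actors.
; When destroyed, the bullet calls BulletDestroyed on its owning drone.
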(event `self.ReceiveBeginPlay`)

(event `self.ReceiveTick`
  (params (DeltaSeconds :type "Float (single-precision)"))
  (`self.K2_SetActorLocation` (+ (`self.K2_GetActorLocation`) (* (`self.speed`) (`GameplayStatics.GetWorldDeltaSeconds`) (`self.GetActorForwardVector`))))
  (`self.K2_SetActorRotation` (`self.K2_GetActorRotation` (`self.GetOwner`))))

(event `self.ReceiveDestroyed`
  (bind _asbp_player_drone (cast `/Game/Blueprints/BP_PlayerDrone` (`self.GetOwner`)))
  (`/Game/Blueprints/BP_PlayerDrone.BulletDestroyed` _asbp_player_drone))

(event `self.Capsule.OnComponentBeginOverlap`
  (params (OverlappedComponent :type "PrimitiveComponent Object Reference") (OtherActor :type "Actor Object Reference") (OtherComp :type "PrimitiveComponent Object Reference") (OtherBodyIndex :type Integer) (bFromSweep :type Boolean) (SweepResult :type "HitResult Structure (by ref)"))
  (if (`self.ActorHasTag` OtherActor "PlayerTwoBullet")
    (`self.K2_DestroyActor` OtherActor)
    (`self.K2_DestroyActor`)
    (elif (`self.ActorHasTag` OtherActor "PlayerTwo")
      (`self.K2_DestroyActor` OtherActor)
      (`self.K2_DestroyActor`))))

(fn `UserConstructionScript`)
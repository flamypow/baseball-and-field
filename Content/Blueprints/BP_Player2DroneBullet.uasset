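; BP_Player2DroneBullet is the bullet belonging to Player 2's drone in a two-player game.
; When its capsule begins overlapping an actor tagged as Player One or a Player One bullet, it destroys both that actor and itself.
; On destruction, it casts its owner to BP_Player2Drone and calls P2BulletDestroyed to notify the drone.
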(event `self.ReceiveDestroyed`
  (bind _asbp_player_2drone (cast `/Game/Blueprints/BP_Player2Drone` (`self.GetOwner`)))
  (`/Game/Blueprints/BP_Player2Drone.P2BulletDestroyed` _asbp_player_2drone))

(event `self.Capsule.OnComponentBeginOverlap`
  (params (OverlappedComponent :type "PrimitiveComponent Object Reference") (OtherActor :type "Actor Object Reference") (OtherComp :type "PrimitiveComponent Object Reference") (OtherBodyIndex :type Integer) (bFromSweep :type Boolean) (SweepResult :type "HitResult Structure (by ref)"))
  (if (`self.ActorHasTag` OtherActor "PlayerOneBullet")
    (`self.K2_DestroyActor` OtherActor)
    (`self.K2_DestroyActor`)
    (elif (`self.ActorHasTag` OtherActor "PlayerOne")
      (`self.K2_DestroyActor` OtherActor)
      (`self.K2_DestroyActor`))))

(fn `UserConstructionScript`
  (`parent.UserConstructionScript`))
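; Player 2's drone pawn, which turns in four directions, fires bullets and reports its destruction through CallPlayerDestroyed.
; P1-named input actions and P2 direction events share logic: a perpendicular direction turns it, the opposite is ignored, and the current facing fires.
; Four identical bullet routines spawn a timed bullet, with P2BulletInPlay blocking further shots until P2BulletDestroyed clears it.
; Capsule overlap with a PlayerOne-tagged actor destroys both.
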(event `EnhancedInput|/Game/Input/IA_UpPressedP1`
  (params (ActionValue :type Boolean) (ElapsedSeconds :type "Float (double-precision)") (TriggeredSeconds :type "Float (double-precision)") (InputAction :type "InputAction Object Reference" :default "/Game/Input/IA_UpPressedP1.IA_UpPressedP1"))
  (:`Triggered`
    (if (== (`self.K2_GetActorRotation`) (struct)) :!label _label
      (if (not (`self.P2BulletInPlay`))
        (set `self.P2BulletInPlay` true)
        (bind _returnvalue (`|SpawnActorFromClass` "/Game/Blueprints/BP_Player2DroneBullet.BP_Player2DroneBullet_C" (`self.GetTransform`) "AlwaysSpawn" "MultiplyWithRoot" null null))
        (`self.SetOwner` _returnvalue self)
        (`KismetSystemLibrary.Delay` (`self.Duration`))
        (`self.K2_DestroyActor` _returnvalue))
      (elif (not (== (`self.K2_GetActorRotation`) (struct :`Yaw` 180.0)))
        (`self.K2_SetActorRotation` (struct))))))

(event `P2Up`
  (goto _label))

(event `EnhancedInput|/Game/Input/IA_DownPressedP1`
  (params (ActionValue :type Boolean) (ElapsedSeconds :type "Float (double-precision)") (TriggeredSeconds :type "Float (double-precision)") (InputAction :type "InputAction Object Reference" :default "/Game/Input/IA_DownPressedP1.IA_DownPressedP1"))
  (:`Triggered`
    (if (== (`self.K2_GetActorRotation`) (struct :`Yaw` 180.0)) :!label _label_2
      (if (not (`self.P2BulletInPlay`))
        (set `self.P2BulletInPlay` true)
        (bind _returnvalue (`|SpawnActorFromClass` "/Game/Blueprints/BP_Player2DroneBullet.BP_Player2DroneBullet_C" (`self.GetTransform`) "AlwaysSpawn" "MultiplyWithRoot" null null))
        (`self.SetOwner` _returnvalue self)
        (`KismetSystemLibrary.Delay` (`self.Duration`))
        (`self.K2_DestroyActor` _returnvalue))
      (elif (not (== (`self.K2_GetActorRotation`) (struct)))
        (`self.K2_SetActorRotation` (struct :`Yaw` 180.0))))))

(event `P2Down`
  (goto _label_2))

(event `EnhancedInput|/Game/Input/IA_LeftPressedP1`
  (params (ActionValue :type Boolean) (ElapsedSeconds :type "Float (double-precision)") (TriggeredSeconds :type "Float (double-precision)") (InputAction :type "InputAction Object Reference" :default "/Game/Input/IA_LeftPressedP1.IA_LeftPressedP1"))
  (:`Triggered`
    (if (== (`self.K2_GetActorRotation`) (struct :`Yaw` 270.0)) :!label _label_3
      (if (not (`self.P2BulletInPlay`))
        (set `self.P2BulletInPlay` true)
        (bind _returnvalue (`|SpawnActorFromClass` "/Game/Blueprints/BP_Player2DroneBullet.BP_Player2DroneBullet_C" (`self.GetTransform`) "AlwaysSpawn" "MultiplyWithRoot" null null))
        (`self.SetOwner` _returnvalue self)
        (`KismetSystemLibrary.Delay` (`self.Duration`))
        (`self.K2_DestroyActor` _returnvalue))
      (elif (not (== (`self.K2_GetActorRotation`) (struct :`Yaw` 90.0)))
        (`self.K2_SetActorRotation` (struct :`Yaw` 270.0))))))

(event `P2Left`
  (goto _label_3))

(event `EnhancedInput|/Game/Input/IA_RightPressedP1`
  (params (ActionValue :type Boolean) (ElapsedSeconds :type "Float (double-precision)") (TriggeredSeconds :type "Float (double-precision)") (InputAction :type "InputAction Object Reference" :default "/Game/Input/IA_RightPressedP1.IA_RightPressedP1"))
  (:`Triggered`
    (if (== (`self.K2_GetActorRotation`) (struct :`Yaw` 90.0)) :!label _label_4
      (if (not (`self.P2BulletInPlay`))
        (set `self.P2BulletInPlay` true)
        (bind _returnvalue (`|SpawnActorFromClass` "/Game/Blueprints/BP_Player2DroneBullet.BP_Player2DroneBullet_C" (`self.GetTransform`) "AlwaysSpawn" "MultiplyWithRoot" null null))
        (`self.SetOwner` _returnvalue self)
        (`KismetSystemLibrary.Delay` (`self.Duration`))
        (`self.K2_DestroyActor` _returnvalue))
      (elif (not (== (`self.K2_GetActorRotation`) (struct :`Yaw` 270.0)))
        (`self.K2_SetActorRotation` (struct :`Yaw` 90.0))))))

(event `P2Right`
  (goto _label_4))

(event `P2BulletDestroyed`
  (set `self.P2BulletInPlay` false))

(event `self.ReceiveDestroyed`
  (`self.PlayerDestroyed`))

(event `self.Capsule.OnComponentBeginOverlap`
  (params (OverlappedComponent :type "PrimitiveComponent Object Reference") (OtherActor :type "Actor Object Reference") (OtherComp :type "PrimitiveComponent Object Reference") (OtherBodyIndex :type Integer) (bFromSweep :type Boolean) (SweepResult :type "HitResult Structure (by ref)"))
  (if (`self.ActorHasTag` OtherActor "PlayerOne")
    (`self.K2_DestroyActor` OtherActor)
    (`self.K2_DestroyActor`)))

(fn `UserConstructionScript`
  (`parent.UserConstructionScript`))